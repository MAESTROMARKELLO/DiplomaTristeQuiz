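; Quiz room actor for level 4 that slides two doors, plays host audio and shows a question when the player enters.
; Four answer zones enable Interact; only the first is correct, reversing the doors, while others cost a life, eventually triggering the death screen.
; Leaving after answering shows the To Be Continued widget.
; A separate box overlap temporarily swaps two walls' material and WorldStatic collision response.
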(event `self.AnswerCollider.OnComponentBeginOverlap`
  (params (OverlappedComponent :type "PrimitiveComponent Object Reference") (OtherActor :type "Actor Object Reference") (OtherComp :type "PrimitiveComponent Object Reference") (OtherBodyIndex :type Integer) (bFromSweep :type Boolean) (SweepResult :type "HitResult Structure (by ref)"))
  ;[0 0.5255 1 1 132] Answer logic
  (if (not (`self.Answered`))
    (`/Engine/EditorBlueprintResources/StandardMacros.DoOnce` false :!label _label
      (:`Completed`
        (`/Game/MarkS/UIX/MainWidget.ShowAnswerMessage` (`self.MainWidget`))
        (cast `Character` OtherActor)
        (`self.EnableInput` (`GameplayStatics.GetPlayerController` 0))))))

(event `self.QuestionCollider.OnComponentBeginOverlap`
  (params (OverlappedComponent :type "PrimitiveComponent Object Reference") (OtherActor :type "Actor Object Reference") (OtherComp :type "PrimitiveComponent Object Reference") (OtherBodyIndex :type Integer) (bFromSweep :type Boolean) (SweepResult :type "HitResult Structure (by ref)"))
  ;[0.9643 1 0 1 117] Question logic
  (if (`self.Answered`)
    _
    (elif (`PrimitiveComponent.IsOverlappingActor` (`self.QuestionCollider`) (`GameplayStatics.GetPlayerCharacter` 0))
      (`/Engine/EditorBlueprintResources/StandardMacros.DoOnce` false :!label _label_2
        (:`Completed`
          (`|ExecutionSequence`
            (:`then_0`
              (bind (_outdoor _relativerotation _returnvalue) (`self.OpenCloseDoor` true (`self.DoorIn`)))
              (`GameplayStatics.PlaySoundAtLocation` "/Game/MarkS/Sounds/DoorOpen.DoorOpen" _returnvalue (struct) 1.0 1.0 2.0 null null null)
              (`KismetSystemLibrary.MoveComponentTo` _outdoor _returnvalue _relativerotation false false 1.5))
            (:`then_1`
              (bind (_outdoor_2 _relativerotation_2 _returnvalue_2) (`self.OpenCloseDoor` true (`self.DoorOut`)))
              (`GameplayStatics.PlaySoundAtLocation` "/Game/MarkS/Sounds/DoorOpen.DoorOpen" _returnvalue_2 (struct) 1.0 1.0 2.0 null null null)
              (`KismetSystemLibrary.MoveComponentTo` _outdoor_2 _returnvalue_2 _relativerotation_2 false false 1.5))
            (:`then_2`
              (bind _outactors (`GameplayStatics.GetAllActorsOfClass` "/Game/MarkS/Characters/FirstPersonCharacter.FirstPersonCharacter_C"))
              (set `self.MainWidget` (`/Game/MarkS/Characters/FirstPersonCharacter.Widget` (`|GetArrayItem` _outactors)))
              (`KismetSystemLibrary.Delay` 1.5)
              (bind _outactors_2 (`GameplayStatics.GetAllActorsOfClass` "/Game/MarkS/Characters/FirstPersonCharacter.FirstPersonCharacter_C"))
              (`GameplayStatics.PlaySoundAtLocation` "/Game/MarkS/Sounds/lvl4.lvl4" (`SceneComponent.K2_GetComponentLocation` (`Character.Mesh` (`/Game/MarkS/Characters/FirstPersonCharacter.Host` (`|GetArrayItem` _outactors_2)))) (struct) 1.0 1.0 0.0 null null null))
            (:`then_3`
              (`/Game/MarkS/UIX/MainWidget.ShowQuestion` (`self.MainWidget`)))))))))

(event `self.AnswerCollider2.OnComponentBeginOverlap`
  (params (OverlappedComponent :type "PrimitiveComponent Object Reference") (OtherActor :type "Actor Object Reference") (OtherComp :type "PrimitiveComponent Object Reference") (OtherBodyIndex :type Integer) (bFromSweep :type Boolean) (SweepResult :type "HitResult Structure (by ref)"))
  ;[0 0.5255 1 1 132] Answer logic
  (if (not (`self.Answered`))
    (`/Engine/EditorBlueprintResources/StandardMacros.DoOnce` false :!label _label_3
      (:`Completed`
        (`/Game/MarkS/UIX/MainWidget.ShowAnswerMessage` (`self.MainWidget`))
        (cast `Character` OtherActor)
        (`self.EnableInput` (`GameplayStatics.GetPlayerController` 0))))))

(event `self.AnswerCollider2.OnComponentEndOverlap`
  (params (OverlappedComponent :type "PrimitiveComponent Object Reference") (OtherActor :type "Actor Object Reference") (OtherComp :type "PrimitiveComponent Object Reference") (OtherBodyIndex :type Integer))
  ;[0 0.5255 1 1 132] Answer logic
  (`/Game/MarkS/UIX/MainWidget.HideAnswerMessage` (`self.MainWidget`))
  (cast `Character` OtherActor)
  (`self.DisableInput` (`GameplayStatics.GetPlayerController` 0))
  (goto _label_3 :!via `Reset`))

(event `self.AnswerCollider.OnComponentEndOverlap`
  (params (OverlappedComponent :type "PrimitiveComponent Object Reference") (OtherActor :type "Actor Object Reference") (OtherComp :type "PrimitiveComponent Object Reference") (OtherBodyIndex :type Integer))
  ;[0 0.5255 1 1 132] Answer logic
  (`/Game/MarkS/UIX/MainWidget.HideAnswerMessage` (`self.MainWidget`))
  (cast `Character` OtherActor)
  (`self.DisableInput` (`GameplayStatics.GetPlayerController` 0))
  (goto _label :!via `Reset`))

(event `self.QuestionCollider.OnComponentEndOverlap`
  (params (OverlappedComponent :type "PrimitiveComponent Object Reference") (OtherActor :type "Actor Object Reference") (OtherComp :type "PrimitiveComponent Object Reference") (OtherBodyIndex :type Integer))
  ;[0.9643 1 0 1 117] Question logic
  (if (`self.Answered`)
    (bind _returnvalue (`|CreateWidget` "/Game/MarkS/UIX/ToBeContinuedWidget.ToBeContinuedWidget_C"))
    (`UserWidget.AddToViewport` _returnvalue 0)
    (set `PlayerController.bShowMouseCursor` true (`GameplayStatics.GetPlayerController` 0))))

(event `self.AnswerCollider3.OnComponentBeginOverlap`
  (params (OverlappedComponent :type "PrimitiveComponent Object Reference") (OtherActor :type "Actor Object Reference") (OtherComp :type "PrimitiveComponent Object Reference") (OtherBodyIndex :type Integer) (bFromSweep :type Boolean) (SweepResult :type "HitResult Structure (by ref)"))
  ;[0 0.5255 1 1 132] Answer logic
  (if (not (`self.Answered`))
    (`/Engine/EditorBlueprintResources/StandardMacros.DoOnce` false :!label _label_4
      (:`Completed`
        (`/Game/MarkS/UIX/MainWidget.ShowAnswerMessage` (`self.MainWidget`))
        (cast `Character` OtherActor)
        (`self.EnableInput` (`GameplayStatics.GetPlayerController` 0))))))

(event `self.AnswerCollider4.OnComponentBeginOverlap`
  (params (OverlappedComponent :type "PrimitiveComponent Object Reference") (OtherActor :type "Actor Object Reference") (OtherComp :type "PrimitiveComponent Object Reference") (OtherBodyIndex :type Integer) (bFromSweep :type Boolean) (SweepResult :type "HitResult Structure (by ref)"))
  ;[0 0.5255 1 1 132] Answer logic
  (if (not (`self.Answered`))
    (`/Engine/EditorBlueprintResources/StandardMacros.DoOnce` false :!label _label_5
      (:`Completed`
        (`/Game/MarkS/UIX/MainWidget.ShowAnswerMessage` (`self.MainWidget`))
        (cast `Character` OtherActor)
        (`self.EnableInput` (`GameplayStatics.GetPlayerController` 0))))))

(event `InputAction|Interact`
  (params (Key :type "Key Structure"))
  (bind _mainwidget (`self.MainWidget`))
  (bind _returnvalue (`self.K2_GetActorLocation` (`GameplayStatics.GetPlayerCharacter` 0)))
  ;[0.9643 1 0 1 117] Question logic
  (:`Pressed`
    (`GameplayStatics.PlaySoundAtLocation` "/Game/MarkS/Sounds/ButtonPressed.ButtonPressed" _returnvalue (struct) 1.0 1.0 0.0 null null null)
    (`KismetSystemLibrary.Delay` 1.0)
    (if (`PrimitiveComponent.IsOverlappingActor` (`self.AnswerCollider`) (`GameplayStatics.GetPlayerCharacter` 0))
      (if (not (`self.Answered`))
        (`GameplayStatics.PlaySoundAtLocation` "/Game/MarkS/Sounds/rightAnswer.rightAnswer" _returnvalue (struct) 1.0 1.0 0.0 null null null)
        (`KismetSystemLibrary.Delay` 0.5)
        (`|ExecutionSequence`
          (:`then_0`
            (bind (_outdoor _relativerotation _returnvalue_2) (`self.OpenCloseDoor` false (`self.DoorOut`)))
            (`GameplayStatics.PlaySoundAtLocation` "/Game/MarkS/Sounds/DoorOpen.DoorOpen" _returnvalue_2 (struct) 1.0 1.0 2.0 null null null)
            (`KismetSystemLibrary.MoveComponentTo` _outdoor _returnvalue_2 _relativerotation false false 1.5))
          (:`then_1`
            (bind (_outdoor_2 _relativerotation_2 _returnvalue_3) (`self.OpenCloseDoor` false (`self.DoorIn`)))
            (`GameplayStatics.PlaySoundAtLocation` "/Game/MarkS/Sounds/DoorOpen.DoorOpen" _returnvalue_3 (struct) 1.0 1.0 2.0 null null null)
            (`KismetSystemLibrary.MoveComponentTo` _outdoor_2 _returnvalue_3 _relativerotation_2 false false 1.5))
          (:`then_2`
            (`/Game/MarkS/UIX/MainWidget.ShowRightMessage` (`self.MainWidget`))
            (`self.DisableInput` (`GameplayStatics.GetPlayerController` 0))
            (set `self.Answered` true))))
      (else
        (`GameplayStatics.PlaySoundAtLocation` "/Game/MarkS/Sounds/wrongAnswer.wrongAnswer" _returnvalue (struct) 1.0 1.0 0.0 null null null)
        (`KismetSystemLibrary.Delay` 0.5)
        (`|ExecutionSequence`
          (:`then_0`
            (bind _outactors (`GameplayStatics.GetAllActorsOfClass` "/Game/MarkS/Characters/FirstPersonCharacter.FirstPersonCharacter_C"))
            (bind _output (`|GetArrayItem` _outactors))
            (set `/Game/MarkS/Characters/FirstPersonCharacter.Lives` (- (`/Game/MarkS/Characters/FirstPersonCharacter.Lives` _output) 1) _output))
          (:`then_1`
            (if (== (`/Game/MarkS/Characters/FirstPersonCharacter.Lives` _output) 1)
              (`/Game/MarkS/UIX/MainWidget.ShowWrongMessage` _mainwidget)
              (elif (== (`/Game/MarkS/Characters/FirstPersonCharacter.Lives` _output) 2)
                (`/Game/MarkS/UIX/MainWidget.ShowWrongMessage` _mainwidget)
                (else
                  (`self.K2_DestroyActor` (`GameplayStatics.GetPlayerCharacter` 0))
                  (set `PlayerController.bShowMouseCursor` true (`GameplayStatics.GetPlayerController` 0))
                  (`/Game/MarkS/UIX/MainWidget.ShowDeathScreen` _mainwidget)
                  (set `self.WrongAnswers` 0)
                  (`|ExecutionSequence`
                    (:`then_1`
                      (`self.K2_DestroyActor`))
                    (:`then_2`
                      (goto _label_2 :!via `Reset`))))))))))))

(event `self.AnswerCollider4.OnComponentEndOverlap`
  (params (OverlappedComponent :type "PrimitiveComponent Object Reference") (OtherActor :type "Actor Object Reference") (OtherComp :type "PrimitiveComponent Object Reference") (OtherBodyIndex :type Integer))
  ;[0 0.5255 1 1 132] Answer logic
  (`/Game/MarkS/UIX/MainWidget.HideAnswerMessage` (`self.MainWidget`))
  (cast `Character` OtherActor)
  (`self.DisableInput` (`GameplayStatics.GetPlayerController` 0))
  (goto _label_5 :!via `Reset`))

(event `self.AnswerCollider3.OnComponentEndOverlap`
  (params (OverlappedComponent :type "PrimitiveComponent Object Reference") (OtherActor :type "Actor Object Reference") (OtherComp :type "PrimitiveComponent Object Reference") (OtherBodyIndex :type Integer))
  ;[0 0.5255 1 1 132] Answer logic
  (`/Game/MarkS/UIX/MainWidget.HideAnswerMessage` (`self.MainWidget`))
  (cast `Character` OtherActor)
  (`self.DisableInput` (`GameplayStatics.GetPlayerController` 0))
  (goto _label_4 :!via `Reset`))

(event `self.Box.OnComponentBeginOverlap`
  (params (OverlappedComponent :type "PrimitiveComponent Object Reference") (OtherActor :type "Actor Object Reference") (OtherComp :type "PrimitiveComponent Object Reference") (OtherBodyIndex :type Integer) (bFromSweep :type Boolean) (SweepResult :type "HitResult Structure (by ref)"))
  (bind _wall1 (`self.Wall1`))
  (bind _wall2 (`self.Wall2`))
  ;[0 0.5255 1 1 132] Answer logic
  (`|ExecutionSequence`
    (:`then_0`
      (`PrimitiveComponent.SetMaterial` _wall1 0 "/Game/MarkS/Materials/wallmaterial.wallmaterial")
      (`PrimitiveComponent.SetCollisionResponseToChannel` _wall1 "ECC_WorldStatic" "ECR_Ignore"))
    (:`then_1`
      (`PrimitiveComponent.SetMaterial` _wall2 0 "/Game/MarkS/Materials/wallmaterial.wallmaterial")
      (`PrimitiveComponent.SetCollisionResponseToChannel` _wall2 "ECC_WorldStatic" "ECR_Ignore"))))

(event `self.Box.OnComponentEndOverlap`
  (params (OverlappedComponent :type "PrimitiveComponent Object Reference") (OtherActor :type "Actor Object Reference") (OtherComp :type "PrimitiveComponent Object Reference") (OtherBodyIndex :type Integer))
  (bind _wall1 (`self.Wall1`))
  (bind _wall2 (`self.Wall2`))
  ;[0 0.5255 1 1 132] Answer logic
  (`|ExecutionSequence`
    (:`then_0`
      (`PrimitiveComponent.SetMaterial` _wall1 0 "/Game/Geometry/Meshes/CubeMaterial.CubeMaterial")
      (`PrimitiveComponent.SetCollisionResponseToChannel` _wall1 "ECC_WorldStatic" "ECR_Block"))
    (:`then_1`
      (`PrimitiveComponent.SetMaterial` _wall2 0 "/Game/Geometry/Meshes/CubeMaterial.CubeMaterial")
      (`PrimitiveComponent.SetCollisionResponseToChannel` _wall2 "ECC_WorldStatic" "ECR_Block"))))

(fn `OpenCloseDoor`
  (params (Open :type Boolean) (Door :type "StaticMeshComponent Object Reference"))
  (returns (OutDoor :type "StaticMeshComponent Object Reference") (RelativeRotation :type "Rotator Structure") (ReturnValue :type "Vector Structure"))
  (bind (_relativelocation_x _relativelocation_y _relativelocation_z) (`KismetMathLibrary.BreakVector` (`SceneComponent.RelativeLocation` Door)))
  (bind (_relativelocation_x_2 _relativelocation_y_2 _relativelocation_z_2) (`KismetMathLibrary.BreakVector` (`SceneComponent.RelativeLocation` Door)))
  (bind _relativerotation (`SceneComponent.RelativeRotation` Door))
  (if Open
    (return Door _relativerotation (`KismetMathLibrary.MakeVector` (+ (`self.MoveDistance`) _relativelocation_x_2) _relativelocation_y_2 _relativelocation_z_2))
    (else
      (return Door _relativerotation (`KismetMathLibrary.MakeVector` (- _relativelocation_x (`self.MoveDistance`)) _relativelocation_y _relativelocation_z)))))

(fn `UserConstructionScript`)