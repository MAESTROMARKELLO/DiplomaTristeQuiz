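; Question room actor that slides both doors on entry, shows a question, and slides them back once solved.
; Four boxes track the AnswerCube as Block, which Interact at AnswerCollider1 passes to the widget's rotation puzzle; passing its check arms the answer colliders.
; Colliders toggle input and prompts through DoOnce gates.
; AnswerCollider4 is correct, advancing progression, weapon and host; other answers cost lives, ending in a death screen.
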(event `self.QuestionCollider.OnComponentBeginOverlap`
  (params (OverlappedComponent :type "PrimitiveComponent Object Reference") (OtherActor :type "Actor Object Reference") (OtherComp :type "PrimitiveComponent Object Reference") (OtherBodyIndex :type Integer) (bFromSweep :type Boolean) (SweepResult :type "HitResult Structure (by ref)"))
  (bind _mainwidget (`self.MainWidget`))
  (bind _mainwidget_2 (`self.MainWidget`))
  (bind _mainwidget_3 (`self.MainWidget`))
  (bind _mainwidget_4 (`self.MainWidget`))
  (if (`self.Answered`)
    _
    (elif (`PrimitiveComponent.IsOverlappingActor` (`self.QuestionCollider`) (`GameplayStatics.GetPlayerCharacter` 0))
      (`/Engine/EditorBlueprintResources/StandardMacros.DoOnce` false :!label _label
        (:`Completed`
          (`|ExecutionSequence`
            (:`then_0`
              (bind (_outdoor _relativerotation _returnvalue) (`self.OpenCloseDoor` true (`self.DoorIn`)))
              (`GameplayStatics.PlaySoundAtLocation` "/Game/MarkS/Sounds/DoorOpen.DoorOpen" _returnvalue (struct) 1.0 1.0 2.0 null null null)
              (`KismetSystemLibrary.MoveComponentTo` _outdoor _returnvalue _relativerotation false false 1.5))
            (:`then_1`
              (bind (_outdoor_2 _relativerotation_2 _returnvalue_2) (`self.OpenCloseDoor` true (`self.DoorOut`)))
              (`GameplayStatics.PlaySoundAtLocation` "/Game/MarkS/Sounds/DoorOpen.DoorOpen" _returnvalue_2 (struct) 1.0 1.0 2.0 null null null)
              (`KismetSystemLibrary.MoveComponentTo` _outdoor_2 _returnvalue_2 _relativerotation_2 false false 1.5))
            (:`then_2`
              (bind _outactors (`GameplayStatics.GetAllActorsOfClass` "/Game/MarkS/Characters/FirstPersonCharacter.FirstPersonCharacter_C"))
              (bind _output_get (set `self.MainWidget` (`/Game/MarkS/Characters/FirstPersonCharacter.Widget` (`|GetArrayItem` _outactors))))
              (`/Game/MarkS/UIX/MainWidget.ShowQuestion` _output_get)
              (`/Game/MarkS/UIX/MainWidget.ShowHUD` _output_get)
              (`KismetSystemLibrary.Delay` 1.5)
              (bind _outactors_2 (`GameplayStatics.GetAllActorsOfClass` "/Game/MarkS/Characters/FirstPersonCharacter.FirstPersonCharacter_C"))
              (`GameplayStatics.PlaySoundAtLocation` "/Game/MarkS/Sounds/lvl3.lvl3" (`SceneComponent.K2_GetComponentLocation` (`Character.Mesh` (`/Game/MarkS/Characters/FirstPersonCharacter.Host` (`|GetArrayItem` _outactors_2)))) (struct) 1.0 1.0 0.0 null null null)
              (`|ExecutionSequence`
                (:`then_0`
                  (goto _label_2 :!via `Reset`))
                (:`then_1`
                  (goto _label_3 :!via `Reset`))
                (:`then_2`
                  (goto _label_4 :!via `Reset`))
                (:`then_3`
                  (goto _label_5 :!via `Reset`))))))))))

(event `self.AnswerCollider.OnComponentBeginOverlap`
  (params (OverlappedComponent :type "PrimitiveComponent Object Reference") (OtherActor :type "Actor Object Reference") (OtherComp :type "PrimitiveComponent Object Reference") (OtherBodyIndex :type Integer) (bFromSweep :type Boolean) (SweepResult :type "HitResult Structure (by ref)"))
  (bind _mainwidget (`self.MainWidget`))
  (if (`self.Placed`)
    (if (not (`self.Answered`))
      (`/Engine/EditorBlueprintResources/StandardMacros.DoOnce` false :!label _label_2
        (:`Completed`
          (`/Engine/EditorBlueprintResources/StandardMacros.IsValid` _mainwidget
            (:`Is Valid`
              (`/Game/MarkS/UIX/MainWidget.ShowAnswerMessage` _mainwidget)
              (cast `Character` OtherActor)
              (`self.EnableInput` (`GameplayStatics.GetPlayerController` 0)))))))))

(event `self.AnswerCollider2.OnComponentBeginOverlap`
  (params (OverlappedComponent :type "PrimitiveComponent Object Reference") (OtherActor :type "Actor Object Reference") (OtherComp :type "PrimitiveComponent Object Reference") (OtherBodyIndex :type Integer) (bFromSweep :type Boolean) (SweepResult :type "HitResult Structure (by ref)"))
  (bind _mainwidget (`self.MainWidget`))
  (if (`self.Placed`)
    (if (not (`self.Answered`))
      (`/Engine/EditorBlueprintResources/StandardMacros.DoOnce` false :!label _label_3
        (:`Completed`
          (`/Engine/EditorBlueprintResources/StandardMacros.IsValid` _mainwidget
            (:`Is Valid`
              (`/Game/MarkS/UIX/MainWidget.ShowAnswerMessage` _mainwidget)
              (cast `Character` OtherActor)
              (`self.EnableInput` (`GameplayStatics.GetPlayerController` 0)))))))))

(event `self.AnswerCollider2.OnComponentEndOverlap`
  (params (OverlappedComponent :type "PrimitiveComponent Object Reference") (OtherActor :type "Actor Object Reference") (OtherComp :type "PrimitiveComponent Object Reference") (OtherBodyIndex :type Integer))
  (if (`self.Placed`)
    (`/Game/MarkS/UIX/MainWidget.HideAnswerMessage` (`self.MainWidget`))
    (`|ExecutionSequence`
      (:`then_0`
        (goto _label_3 :!via `Reset`))
      (:`then_1`
        (cast `Character` OtherActor)
        (`self.DisableInput` (`GameplayStatics.GetPlayerController` 0))))))

(event `self.AnswerCollider.OnComponentEndOverlap`
  (params (OverlappedComponent :type "PrimitiveComponent Object Reference") (OtherActor :type "Actor Object Reference") (OtherComp :type "PrimitiveComponent Object Reference") (OtherBodyIndex :type Integer))
  (if (`self.Placed`)
    (`/Game/MarkS/UIX/MainWidget.HideAnswerMessage` (`self.MainWidget`))
    (`|ExecutionSequence`
      (:`then_0`
        (goto _label_2 :!via `Reset`))
      (:`then_1`
        (cast `Character` OtherActor)
        (`self.DisableInput` (`GameplayStatics.GetPlayerController` 0))))))

(event `InputAction|Interact`
  (params (Key :type "Key Structure"))
  (bind _mainwidget (`self.MainWidget`))
  (bind _mainwidget_2 (`self.MainWidget`))
  (bind _mainwidget_3 (`self.MainWidget`))
  (bind _returnvalue (`self.K2_GetActorLocation` (`GameplayStatics.GetPlayerCharacter` 0)))
  (:`Pressed`
    (if (`self.Placed`)
      (`GameplayStatics.PlaySoundAtLocation` "/Game/MarkS/Sounds/ButtonPressed.ButtonPressed" _returnvalue (struct) 1.0 1.0 0.0 null null null)
      (`KismetSystemLibrary.Delay` 1.0)
      (if (`PrimitiveComponent.IsOverlappingActor` (`self.AnswerCollider4`) (`GameplayStatics.GetPlayerCharacter` 0))
        (if (not (`self.Answered`))
          (`GameplayStatics.PlaySoundAtLocation` "/Game/MarkS/Sounds/rightAnswer.rightAnswer" _returnvalue (struct) 1.0 1.0 0.0 null null null)
          (`KismetSystemLibrary.Delay` 0.5)
          (`|ExecutionSequence`
            (:`then_0`
              (bind (_outdoor _relativerotation _returnvalue_2) (`self.OpenCloseDoor` false (`self.DoorIn`)))
              (`GameplayStatics.PlaySoundAtLocation` "/Game/MarkS/Sounds/DoorOpen.DoorOpen" _returnvalue_2 (struct) 1.0 1.0 2.0 null null null)
              (`KismetSystemLibrary.MoveComponentTo` _outdoor _returnvalue_2 _relativerotation false false 2.0))
            (:`then_1`
              (bind (_outdoor_2 _relativerotation_2 _returnvalue_3) (`self.OpenCloseDoor` false (`self.DoorOut`)))
              (`GameplayStatics.PlaySoundAtLocation` "/Game/MarkS/Sounds/DoorOpen.DoorOpen" _returnvalue_3 (struct) 1.0 1.0 2.0 null null null)
              (`KismetSystemLibrary.MoveComponentTo` _outdoor_2 _returnvalue_3 _relativerotation_2 false false 1.5))
            (:`then_2`
              (`/Game/MarkS/UIX/MainWidget.ShowRightMessage` (`self.MainWidget`))
              (`self.DisableInput` (`GameplayStatics.GetPlayerController` 0))
              (set `self.Answered` true)
              (bind _outactors (`GameplayStatics.GetAllActorsOfClass` "/Game/MarkS/Characters/FirstPersonCharacter.FirstPersonCharacter_C"))
              (bind _outactors_2 (`GameplayStatics.GetAllActorsOfClass` "/Game/MarkS/Main/MainController.MainController_C"))
              (bind _output (`|GetArrayItem` _outactors_2))
              (set `/Game/MarkS/Main/MainController.HUDStage` (+ (`/Game/MarkS/Main/MainController.HUDStage` _output) 1) _output)
              (`/Game/MarkS/Characters/FirstPersonCharacter.ChangeGun` (`|GetArrayItem` _outactors))
              (bind _outactors_3 (`GameplayStatics.GetAllActorsOfClass` "/Game/MarkS/Main/MainController.MainController_C"))
              (`/Game/MarkS/UIX/MainWidget.HideHUD` _mainwidget)
              (bind _output_2 (`|GetArrayItem` _outactors_3))
              (set `/Game/MarkS/Main/MainController.Levels` (+ (`/Game/MarkS/Main/MainController.Levels` _output_2) 1) _output_2)
              (`/Game/MarkS/UIX/MainWidget.ShowHUD` _mainwidget)
              (`/Game/MarkS/UIX/MainWidget.UnlockWeapon` _mainwidget)
              (`KismetSystemLibrary.Delay` 2.0)
              (bind _outactors_4 (`GameplayStatics.GetAllActorsOfClass` "/Game/MarkS/Characters/FirstPersonCharacter.FirstPersonCharacter_C"))
              (`/Game/MarkS/Characters/HostCharacter.NextMove` (`/Game/MarkS/Characters/FirstPersonCharacter.Host` (`|GetArrayItem` _outactors_4))))))
        (else
          (`GameplayStatics.PlaySoundAtLocation` "/Game/MarkS/Sounds/wrongAnswer.wrongAnswer" _returnvalue (struct) 1.0 1.0 0.0 null null null)
          (`KismetSystemLibrary.Delay` 0.5)
          (`|ExecutionSequence`
            (:`then_0`
              (bind _outactors_5 (`GameplayStatics.GetAllActorsOfClass` "/Game/MarkS/Characters/FirstPersonCharacter.FirstPersonCharacter_C"))
              (bind _output_3 (`|GetArrayItem` _outactors_5))
              (set `/Game/MarkS/Characters/FirstPersonCharacter.Lives` (- (`/Game/MarkS/Characters/FirstPersonCharacter.Lives` _output_3) 1) _output_3))
            (:`then_1`
              (if (== (`/Game/MarkS/Characters/FirstPersonCharacter.Lives` _output_3) 2)
                (`/Game/MarkS/UIX/MainWidget.ShowWrongMessage` _mainwidget_3)
                (elif (== (`/Game/MarkS/Characters/FirstPersonCharacter.Lives` _output_3) 1)
                  (`/Game/MarkS/UIX/MainWidget.ShowWrongMessage` _mainwidget_3)
                  (else
                    (`self.K2_DestroyActor` (`GameplayStatics.GetPlayerCharacter` 0))
                    (set `PlayerController.bShowMouseCursor` true (`GameplayStatics.GetPlayerController` 0))
                    (`/Game/MarkS/UIX/MainWidget.ShowDeathScreen` _mainwidget_3)
                    (`|ExecutionSequence`
                      (:`then_1`
                        (`self.K2_DestroyActor`))
                      (:`then_2`
                        (goto _label :!via `Reset`))))))))))
      (elif (`PrimitiveComponent.IsOverlappingActor` (`self.AnswerCollider1`) (`GameplayStatics.GetPlayerCharacter` 0))
        (`/Game/MarkS/UIX/MainWidget.Rotation` _mainwidget_2 (`self.Block`))
        (bind _result (`/Game/MarkS/UIX/MainWidget.Check` _mainwidget_2))
        (if _result
          (set `self.Placed` true)
          (`KismetSystemLibrary.PrintString` "Hello")
          (else
            (set `self.Placed` false)
            (`KismetSystemLibrary.PrintString` "bye")))))))

(event `self.AnswerCollider3.OnComponentBeginOverlap`
  (params (OverlappedComponent :type "PrimitiveComponent Object Reference") (OtherActor :type "Actor Object Reference") (OtherComp :type "PrimitiveComponent Object Reference") (OtherBodyIndex :type Integer) (bFromSweep :type Boolean) (SweepResult :type "HitResult Structure (by ref)"))
  (bind _mainwidget (`self.MainWidget`))
  (if (`self.Placed`)
    (if (not (`self.Answered`))
      (`/Engine/EditorBlueprintResources/StandardMacros.DoOnce` false :!label _label_4
        (:`Completed`
          (`/Engine/EditorBlueprintResources/StandardMacros.IsValid` _mainwidget
            (:`Is Valid`
              (`/Game/MarkS/UIX/MainWidget.ShowAnswerMessage` _mainwidget)
              (cast `Character` OtherActor)
              (`self.EnableInput` (`GameplayStatics.GetPlayerController` 0)))))))))

(event `self.AnswerCollider4.OnComponentBeginOverlap`
  (params (OverlappedComponent :type "PrimitiveComponent Object Reference") (OtherActor :type "Actor Object Reference") (OtherComp :type "PrimitiveComponent Object Reference") (OtherBodyIndex :type Integer) (bFromSweep :type Boolean) (SweepResult :type "HitResult Structure (by ref)"))
  (bind _mainwidget (`self.MainWidget`))
  (if (`self.Placed`)
    (if (not (`self.Answered`))
      (`/Engine/EditorBlueprintResources/StandardMacros.DoOnce` false :!label _label_5
        (:`Completed`
          (`/Engine/EditorBlueprintResources/StandardMacros.IsValid` _mainwidget
            (:`Is Valid`
              (`/Game/MarkS/UIX/MainWidget.ShowAnswerMessage` _mainwidget)
              (cast `Character` OtherActor)
              (`self.EnableInput` (`GameplayStatics.GetPlayerController` 0)))))))))

(event `self.AnswerCollider3.OnComponentEndOverlap`
  (params (OverlappedComponent :type "PrimitiveComponent Object Reference") (OtherActor :type "Actor Object Reference") (OtherComp :type "PrimitiveComponent Object Reference") (OtherBodyIndex :type Integer))
  (if (`self.Placed`)
    (`/Game/MarkS/UIX/MainWidget.HideAnswerMessage` (`self.MainWidget`))
    (`|ExecutionSequence`
      (:`then_0`
        (goto _label_4 :!via `Reset`))
      (:`then_1`
        (cast `Character` OtherActor)
        (`self.DisableInput` (`GameplayStatics.GetPlayerController` 0))))))

(event `self.AnswerCollider4.OnComponentEndOverlap`
  (params (OverlappedComponent :type "PrimitiveComponent Object Reference") (OtherActor :type "Actor Object Reference") (OtherComp :type "PrimitiveComponent Object Reference") (OtherBodyIndex :type Integer))
  (if (`self.Placed`)
    (`/Game/MarkS/UIX/MainWidget.HideAnswerMessage` (`self.MainWidget`))
    (`|ExecutionSequence`
      (:`then_0`
        (goto _label_5 :!via `Reset`))
      (:`then_1`
        (cast `Character` OtherActor)
        (`self.DisableInput` (`GameplayStatics.GetPlayerController` 0))))))

(event `self.AnswerCollider1.OnComponentBeginOverlap`
  (params (OverlappedComponent :type "PrimitiveComponent Object Reference") (OtherActor :type "Actor Object Reference") (OtherComp :type "PrimitiveComponent Object Reference") (OtherBodyIndex :type Integer) (bFromSweep :type Boolean) (SweepResult :type "HitResult Structure (by ref)"))
  (if (not (`self.Answered`))
    (`/Engine/EditorBlueprintResources/StandardMacros.DoOnce` false :!label _label_6
      (:`Completed`
        (`/Game/MarkS/UIX/MainWidget.ShowAnswerMessage` (`self.MainWidget`))
        (cast `Character` OtherActor)
        (`self.EnableInput` (`GameplayStatics.GetPlayerController` 0))))))

(event `self.AnswerCollider1.OnComponentEndOverlap`
  (params (OverlappedComponent :type "PrimitiveComponent Object Reference") (OtherActor :type "Actor Object Reference") (OtherComp :type "PrimitiveComponent Object Reference") (OtherBodyIndex :type Integer))
  (if (not (`self.Answered`))
    (`/Game/MarkS/UIX/MainWidget.HideAnswerMessage` (`self.MainWidget`))
    (cast `Character` OtherActor)
    (`self.DisableInput` (`GameplayStatics.GetPlayerController` 0))
    (goto _label_6 :!via `Reset`)))

(event `self.Box.OnComponentBeginOverlap`
  (params (OverlappedComponent :type "PrimitiveComponent Object Reference") (OtherActor :type "Actor Object Reference") (OtherComp :type "PrimitiveComponent Object Reference") (OtherBodyIndex :type Integer) (bFromSweep :type Boolean) (SweepResult :type "HitResult Structure (by ref)"))
  (if (`PrimitiveComponent.IsOverlappingComponent` (`self.Box`) (`self.AnswerCube`))
    (set `self.Block` 1)))

(event `self.Box1.OnComponentBeginOverlap`
  (params (OverlappedComponent :type "PrimitiveComponent Object Reference") (OtherActor :type "Actor Object Reference") (OtherComp :type "PrimitiveComponent Object Reference") (OtherBodyIndex :type Integer) (bFromSweep :type Boolean) (SweepResult :type "HitResult Structure (by ref)"))
  (if (`PrimitiveComponent.IsOverlappingComponent` (`self.Box1`) (`self.AnswerCube`))
    (set `self.Block` 2)))

(event `self.Box.OnComponentEndOverlap`
  (params (OverlappedComponent :type "PrimitiveComponent Object Reference") (OtherActor :type "Actor Object Reference") (OtherComp :type "PrimitiveComponent Object Reference") (OtherBodyIndex :type Integer))
  (if (not (`PrimitiveComponent.IsOverlappingComponent` (`self.Box`) (`self.AnswerCube`)))
    (set `self.Block` 0)))

(event `self.Box1.OnComponentEndOverlap`
  (params (OverlappedComponent :type "PrimitiveComponent Object Reference") (OtherActor :type "Actor Object Reference") (OtherComp :type "PrimitiveComponent Object Reference") (OtherBodyIndex :type Integer))
  (if (not (`PrimitiveComponent.IsOverlappingComponent` (`self.Box1`) (`self.AnswerCube`)))
    (set `self.Block` 0)))

(event `self.Box2.OnComponentBeginOverlap`
  (params (OverlappedComponent :type "PrimitiveComponent Object Reference") (OtherActor :type "Actor Object Reference") (OtherComp :type "PrimitiveComponent Object Reference") (OtherBodyIndex :type Integer) (bFromSweep :type Boolean) (SweepResult :type "HitResult Structure (by ref)"))
  (if (`PrimitiveComponent.IsOverlappingComponent` (`self.Box2`) (`self.AnswerCube`))
    (set `self.Block` 3)))

(event `self.Box3.OnComponentBeginOverlap`
  (params (OverlappedComponent :type "PrimitiveComponent Object Reference") (OtherActor :type "Actor Object Reference") (OtherComp :type "PrimitiveComponent Object Reference") (OtherBodyIndex :type Integer) (bFromSweep :type Boolean) (SweepResult :type "HitResult Structure (by ref)"))
  (if (`PrimitiveComponent.IsOverlappingComponent` (`self.Box3`) (`self.AnswerCube`))
    (set `self.Block` 4)))

(event `self.Box2.OnComponentEndOverlap`
  (params (OverlappedComponent :type "PrimitiveComponent Object Reference") (OtherActor :type "Actor Object Reference") (OtherComp :type "PrimitiveComponent Object Reference") (OtherBodyIndex :type Integer))
  (if (not (`PrimitiveComponent.IsOverlappingComponent` (`self.Box2`) (`self.AnswerCube`)))
    (set `self.Block` 0)))

(event `self.Box3.OnComponentEndOverlap`
  (params (OverlappedComponent :type "PrimitiveComponent Object Reference") (OtherActor :type "Actor Object Reference") (OtherComp :type "PrimitiveComponent Object Reference") (OtherBodyIndex :type Integer))
  (if (not (`PrimitiveComponent.IsOverlappingComponent` (`self.Box3`) (`self.AnswerCube`)))
    (set `self.Block` 0)))

(fn `OpenCloseDoor`
  (params (Open :type Boolean) (Door :type "StaticMeshComponent Object Reference"))
  (returns (OutDoor :type "StaticMeshComponent Object Reference") (RelativeRotation :type "Rotator Structure") (ReturnValue :type "Vector Structure"))
  (bind (_relativelocation_x _relativelocation_y _relativelocation_z) (`KismetMathLibrary.BreakVector` (`SceneComponent.RelativeLocation` Door)))
  (bind (_relativelocation_x_2 _relativelocation_y_2 _relativelocation_z_2) (`KismetMathLibrary.BreakVector` (`SceneComponent.RelativeLocation` Door)))
  (bind _relativerotation (`SceneComponent.RelativeRotation` Door))
  (if Open
    (return Door _relativerotation (`KismetMathLibrary.MakeVector` (+ (`self.MoveDistance`) _relativelocation_x_2) _relativelocation_y_2 _relativelocation_z_2))
    (else
      (return Door _relativerotation (`KismetMathLibrary.MakeVector` (- _relativelocation_x (`self.MoveDistance`)) _relativelocation_y _relativelocation_z)))))

(fn `UserConstructionScript`)