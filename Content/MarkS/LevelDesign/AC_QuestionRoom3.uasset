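; Puzzle quiz room where cubes on colored buttons unlock four answer spots and the elevator cube triggers moving platforms.
; Entering the question trigger shifts both doors and creates the quiz widget; unlocked answer spots enable Interact input.
; Answer four is correct and moves the exit door back.
; A third wrong answer destroys the player, shows the death screen and returns doors and cubes to their starting positions.
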(event `self.ElevatorStart.OnComponentBeginOverlap`
  (params (OverlappedComponent :type "PrimitiveComponent Object Reference") (OtherActor :type "Actor Object Reference") (OtherComp :type "PrimitiveComponent Object Reference") (OtherBodyIndex :type Integer) (bFromSweep :type Boolean) (SweepResult :type "HitResult Structure (by ref)"))
  (bind _elevator (`self.Elevator`))
  (bind _elevator_2 (`self.Elevator`))
  (bind (_relativelocation_x _relativelocation_y _relativelocation_z) (`KismetMathLibrary.BreakVector` (`SceneComponent.RelativeLocation` _elevator)))
  (bind (_relativelocation_x_2 _relativelocation_y_2 _relativelocation_z_2) (`KismetMathLibrary.BreakVector` (`SceneComponent.RelativeLocation` _elevator_2)))
  ;[1 0 0.1888 1 94] Elevator movement
  (`/Engine/EditorBlueprintResources/StandardMacros.DoOnce` false :!label _label
    (:`Completed`
      (if (`PrimitiveComponent.IsOverlappingComponent` (`self.ElevatorStart`) (`self.ElevatorCube`))
        (`KismetSystemLibrary.Delay` 3.0)
        (`KismetSystemLibrary.MoveComponentTo` _elevator (`KismetMathLibrary.MakeVector` _relativelocation_x _relativelocation_y (+ _relativelocation_z 500.0)) (`SceneComponent.RelativeRotation` _elevator) false false 3.0)
        (`KismetSystemLibrary.Delay` 5.0)
        (`KismetSystemLibrary.MoveComponentTo` _elevator_2 (`KismetMathLibrary.MakeVector` _relativelocation_x_2 _relativelocation_y_2 (+ _relativelocation_z_2 -500.0)) (`SceneComponent.RelativeRotation` _elevator_2) false false 3.0)))))

(event `self.AnswerCollider.OnComponentBeginOverlap`
  (params (OverlappedComponent :type "PrimitiveComponent Object Reference") (OtherActor :type "Actor Object Reference") (OtherComp :type "PrimitiveComponent Object Reference") (OtherBodyIndex :type Integer) (bFromSweep :type Boolean) (SweepResult :type "HitResult Structure (by ref)"))
  ;[0 0.5255 1 1 132] Answer logic
  (if (`self.Answer1Available`)
    (if (not (`self.Answered`))
      (`/Engine/EditorBlueprintResources/StandardMacros.DoOnce` false :!label _label_2
        (:`Completed`
          (`/Game/MarkS/UIX/MainWidget.ShowAnswerMessage` (`self.MainWidget`))
          (cast `Character` OtherActor)
          (`self.EnableInput` (`GameplayStatics.GetPlayerController` 0)))))))

(event `self.QuestionCollider.OnComponentBeginOverlap`
  (params (OverlappedComponent :type "PrimitiveComponent Object Reference") (OtherActor :type "Actor Object Reference") (OtherComp :type "PrimitiveComponent Object Reference") (OtherBodyIndex :type Integer) (bFromSweep :type Boolean) (SweepResult :type "HitResult Structure (by ref)"))
  ;[0.9643 1 0 1 117] Question logic
  (if (`self.Answered`)
    _
    (elif (`PrimitiveComponent.IsOverlappingActor` (`self.QuestionCollider`) (`GameplayStatics.GetPlayerCharacter` 0))
      (`/Engine/EditorBlueprintResources/StandardMacros.DoOnce` false :!label _label_3
        (:`Completed`
          (`|ExecutionSequence`
            (:`then_0`
              (bind (_outdoor _relativerotation _returnvalue) (`self.OpenCloseDoor` true (`self.DoorIn`)))
              (`KismetSystemLibrary.MoveComponentTo` _outdoor _returnvalue _relativerotation false false 1.5))
            (:`then_1`
              (bind (_outdoor_2 _relativerotation_2 _returnvalue_2) (`self.OpenCloseDoor` true (`self.DoorOut`)))
              (`KismetSystemLibrary.MoveComponentTo` _outdoor_2 _returnvalue_2 _relativerotation_2 false false 1.5))
            (:`then_2`
              (bind _returnvalue_3 (`|CreateWidget` "/Game/MarkS/UIX/MainWidget.MainWidget_C"))
              (bind _output_get (set `self.MainWidget` _returnvalue_3))
              (`UserWidget.AddToViewport` _output_get 0))))))))

(event `self.AnswerCollider2.OnComponentBeginOverlap`
  (params (OverlappedComponent :type "PrimitiveComponent Object Reference") (OtherActor :type "Actor Object Reference") (OtherComp :type "PrimitiveComponent Object Reference") (OtherBodyIndex :type Integer) (bFromSweep :type Boolean) (SweepResult :type "HitResult Structure (by ref)"))
  ;[0 0.5255 1 1 132] Answer logic
  (if (`self.Answer2Available`)
    (if (not (`self.Answered`))
      (`/Engine/EditorBlueprintResources/StandardMacros.DoOnce` false :!label _label_4
        (:`Completed`
          (`/Game/MarkS/UIX/MainWidget.ShowAnswerMessage` (`self.MainWidget`))
          (cast `Character` OtherActor)
          (`self.EnableInput` (`GameplayStatics.GetPlayerController` 0)))))))

(event `self.ElevatorStart.OnComponentEndOverlap`
  (params (OverlappedComponent :type "PrimitiveComponent Object Reference") (OtherActor :type "Actor Object Reference") (OtherComp :type "PrimitiveComponent Object Reference") (OtherBodyIndex :type Integer))
  ;[1 0 0.1888 1 94] Elevator movement
  (goto _label :!via `Reset`))

(event `self.AnswerCollider2.OnComponentEndOverlap`
  (params (OverlappedComponent :type "PrimitiveComponent Object Reference") (OtherActor :type "Actor Object Reference") (OtherComp :type "PrimitiveComponent Object Reference") (OtherBodyIndex :type Integer))
  ;[0 0.5255 1 1 132] Answer logic
  (if (`self.Answer2Available`)
    (`/Game/MarkS/UIX/MainWidget.HideAnswerMessage` (`self.MainWidget`))
    (cast `Character` OtherActor)
    (`self.DisableInput` (`GameplayStatics.GetPlayerController` 0))
    (goto _label_4 :!via `Reset`)))

(event `self.AnswerCollider.OnComponentEndOverlap`
  (params (OverlappedComponent :type "PrimitiveComponent Object Reference") (OtherActor :type "Actor Object Reference") (OtherComp :type "PrimitiveComponent Object Reference") (OtherBodyIndex :type Integer))
  ;[0 0.5255 1 1 132] Answer logic
  (if (`self.Answer1Available`)
    (`/Game/MarkS/UIX/MainWidget.HideAnswerMessage` (`self.MainWidget`))
    (cast `Character` OtherActor)
    (`self.DisableInput` (`GameplayStatics.GetPlayerController` 0))
    (goto _label_2 :!via `Reset`)))

(event `self.ElevatorStart3.OnComponentBeginOverlap`
  (params (OverlappedComponent :type "PrimitiveComponent Object Reference") (OtherActor :type "Actor Object Reference") (OtherComp :type "PrimitiveComponent Object Reference") (OtherBodyIndex :type Integer) (bFromSweep :type Boolean) (SweepResult :type "HitResult Structure (by ref)"))
  (bind _elevator3 (`self.Elevator3`))
  (bind (_relativelocation_x _relativelocation_y _relativelocation_z) (`KismetMathLibrary.BreakVector` (`SceneComponent.RelativeLocation` _elevator3)))
  ;[1 0 0.1888 1 94] Elevator movement
  (`/Engine/EditorBlueprintResources/StandardMacros.DoOnce` false
    (:`Completed`
      (if (`PrimitiveComponent.IsOverlappingComponent` (`self.ElevatorStart3`) (`self.ElevatorCube`))
        (`KismetSystemLibrary.Delay` 0.5)
        (`KismetSystemLibrary.MoveComponentTo` _elevator3 (`KismetMathLibrary.MakeVector` (+ _relativelocation_x 1200.0) _relativelocation_y _relativelocation_z) (`SceneComponent.RelativeRotation` _elevator3) false false 3.0)))))

(event `self.ReceiveBeginPlay`
  ;[0.9643 1 0 1 117] Question logic
  (set `self.CubePosition` (`SceneComponent.K2_GetComponentLocation` (`self.ElevatorCube`)))
  (set `self.CubePosition1` (`SceneComponent.K2_GetComponentLocation` (`self.AnswerCube`)))
  (set `self.CubePosition2` (`SceneComponent.K2_GetComponentLocation` (`self.AnswerCube2`)))
  (set `self.CubePosition3` (`SceneComponent.K2_GetComponentLocation` (`self.AnswerCube3`)))
  (set `self.CubePosition4` (`SceneComponent.K2_GetComponentLocation` (`self.AnswerCube4`))))

(event `self.Box2.OnComponentBeginOverlap`
  (params (OverlappedComponent :type "PrimitiveComponent Object Reference") (OtherActor :type "Actor Object Reference") (OtherComp :type "PrimitiveComponent Object Reference") (OtherBodyIndex :type Integer) (bFromSweep :type Boolean) (SweepResult :type "HitResult Structure (by ref)"))
  ;[0 0.5255 1 1 132] Answer logic
  (if (`PrimitiveComponent.IsOverlappingComponent` (`self.Box2`) (`self.AnswerCube2`))
    (set `self.Answer2Available` true)
    (`PrimitiveComponent.SetMaterial` (`self.Button2`) 0 "/Game/MarkS/Materials/Red.Red")))

(event `self.Box.OnComponentBeginOverlap`
  (params (OverlappedComponent :type "PrimitiveComponent Object Reference") (OtherActor :type "Actor Object Reference") (OtherComp :type "PrimitiveComponent Object Reference") (OtherBodyIndex :type Integer) (bFromSweep :type Boolean) (SweepResult :type "HitResult Structure (by ref)"))
  ;[0 0.5255 1 1 132] Answer logic
  (if (`PrimitiveComponent.IsOverlappingComponent` (`self.Box`) (`self.AnswerCube`))
    (set `self.Answer1Available` true)
    (`PrimitiveComponent.SetMaterial` (`self.Button`) 0 "/Game/MarkS/Materials/Red.Red")))

(event `self.ElevatorStart2.OnComponentBeginOverlap`
  (params (OverlappedComponent :type "PrimitiveComponent Object Reference") (OtherActor :type "Actor Object Reference") (OtherComp :type "PrimitiveComponent Object Reference") (OtherBodyIndex :type Integer) (bFromSweep :type Boolean) (SweepResult :type "HitResult Structure (by ref)"))
  (bind _elevator2 (`self.Elevator2`))
  (bind _elevator2_2 (`self.Elevator2`))
  (bind (_relativelocation_x _relativelocation_y _relativelocation_z) (`KismetMathLibrary.BreakVector` (`SceneComponent.RelativeLocation` _elevator2_2)))
  (bind (_relativelocation_x_2 _relativelocation_y_2 _relativelocation_z_2) (`KismetMathLibrary.BreakVector` (`SceneComponent.RelativeLocation` _elevator2)))
  ;[1 0 0.1888 1 94] Elevator movement
  (`/Engine/EditorBlueprintResources/StandardMacros.DoOnce` false :!label _label_5
    (:`Completed`
      (if (`PrimitiveComponent.IsOverlappingComponent` (`self.ElevatorStart2`) (`self.ElevatorCube`))
        (`KismetSystemLibrary.Delay` 2.0)
        (`KismetSystemLibrary.MoveComponentTo` _elevator2_2 (`KismetMathLibrary.MakeVector` _relativelocation_x _relativelocation_y (+ _relativelocation_z 500.0)) (`SceneComponent.RelativeRotation` _elevator2_2) false false 3.0)
        (`KismetSystemLibrary.Delay` 3.0)
        (`KismetSystemLibrary.MoveComponentTo` _elevator2 (`KismetMathLibrary.MakeVector` _relativelocation_x_2 _relativelocation_y_2 (+ _relativelocation_z_2 -500.0)) (`SceneComponent.RelativeRotation` _elevator2) false false 3.0)))))

(event `InputAction|Interact`
  (params (Key :type "Key Structure"))
  (bind _mainwidget (`self.MainWidget`))
  ;[0.9643 1 0 1 117] Question logic
  (:`Pressed`
    (if (`PrimitiveComponent.IsOverlappingActor` (`self.AnswerCollider4`) (`GameplayStatics.GetPlayerCharacter` 0))
      (if (not (`self.Answered`))
        (`/Game/MarkS/UIX/MainWidget.ShowRightMessage` (`self.MainWidget`))
        (bind (_outdoor _relativerotation _returnvalue) (`self.OpenCloseDoor` false (`self.DoorOut`)))
        (`KismetSystemLibrary.MoveComponentTo` _outdoor _returnvalue _relativerotation false false 1.5)
        (`self.DisableInput` (`GameplayStatics.GetPlayerController` 0))
        (set `self.Answered` true))
      (else
        (`|ExecutionSequence`
          (:`then_0`
            (set `self.WrongAnswers` (+ (`self.WrongAnswers`) 1)))
          (:`then_1`
            (if (== (`self.WrongAnswers`) 1)
              (`/Game/MarkS/UIX/MainWidget.ShowWrongMessage` _mainwidget true)
              (elif (== (`self.WrongAnswers`) 2)
                (`/Game/MarkS/UIX/MainWidget.ShowWrongMessage` _mainwidget false)
                (else
                  (`self.K2_DestroyActor` (`GameplayStatics.GetPlayerCharacter` 0))
                  (set `PlayerController.bShowMouseCursor` true (`GameplayStatics.GetPlayerController` 0))
                  (`/Game/MarkS/UIX/MainWidget.ShowDeathScreen` _mainwidget)
                  (set `self.WrongAnswers` 0)
                  (`|ExecutionSequence`
                    (:`then_0`
                      (bind (_outdoor_2 _relativerotation_2 _returnvalue_2) (`self.OpenCloseDoor` false (`self.DoorOut`)))
                      (`KismetSystemLibrary.MoveComponentTo` _outdoor_2 _returnvalue_2 _relativerotation_2 false false 1.5))
                    (:`then_1`
                      (bind (_outdoor_3 _relativerotation_3 _returnvalue_3) (`self.OpenCloseDoor` false (`self.DoorIn`)))
                      (`KismetSystemLibrary.MoveComponentTo` _outdoor_3 _returnvalue_3 _relativerotation_3 false false 1.5))
                    (:`then_2`
                      (goto _label_3 :!via `Reset`))
                    (:`then_3`
                      (`KismetSystemLibrary.MoveComponentTo` (`self.ElevatorCube`) (`self.CubePosition`))
                      (`KismetSystemLibrary.MoveComponentTo` (`self.AnswerCube`) (`self.CubePosition1`) (struct))
                      (`KismetSystemLibrary.MoveComponentTo` (`self.AnswerCube2`) (`self.CubePosition2`))
                      (`KismetSystemLibrary.MoveComponentTo` (`self.AnswerCube3`) (`self.CubePosition3`))
                      (`KismetSystemLibrary.MoveComponentTo` (`self.AnswerCube4`) (`self.CubePosition4`)))))))))))))

(event `self.Box.OnComponentEndOverlap`
  (params (OverlappedComponent :type "PrimitiveComponent Object Reference") (OtherActor :type "Actor Object Reference") (OtherComp :type "PrimitiveComponent Object Reference") (OtherBodyIndex :type Integer))
  ;[0 0.5255 1 1 132] Answer logic
  (if (not (`PrimitiveComponent.IsOverlappingComponent` (`self.Box`) (`self.AnswerCube`)))
    (set `self.Answer1Available` false)
    (`PrimitiveComponent.SetMaterial` (`self.Button`) 0 "/Game/MarkS/Materials/Blue.Blue")))

(event `self.Box2.OnComponentEndOverlap`
  (params (OverlappedComponent :type "PrimitiveComponent Object Reference") (OtherActor :type "Actor Object Reference") (OtherComp :type "PrimitiveComponent Object Reference") (OtherBodyIndex :type Integer))
  ;[0 0.5255 1 1 132] Answer logic
  (if (not (`PrimitiveComponent.IsOverlappingComponent` (`self.Box2`) (`self.AnswerCube2`)))
    (set `self.Answer2Available` false)
    (`PrimitiveComponent.SetMaterial` (`self.Button2`) 0 "/Game/MarkS/Materials/Green.Green")))

(event `self.ElevatorStart2.OnComponentEndOverlap`
  (params (OverlappedComponent :type "PrimitiveComponent Object Reference") (OtherActor :type "Actor Object Reference") (OtherComp :type "PrimitiveComponent Object Reference") (OtherBodyIndex :type Integer))
  ;[1 0 0.1888 1 94] Elevator movement
  (goto _label_5 :!via `Reset`))

(event `self.ElevatorStart4.OnComponentBeginOverlap`
  (params (OverlappedComponent :type "PrimitiveComponent Object Reference") (OtherActor :type "Actor Object Reference") (OtherComp :type "PrimitiveComponent Object Reference") (OtherBodyIndex :type Integer) (bFromSweep :type Boolean) (SweepResult :type "HitResult Structure (by ref)"))
  (bind _elevator4 (`self.Elevator4`))
  (bind _elevator4_2 (`self.Elevator4`))
  (bind (_relativelocation_x _relativelocation_y _relativelocation_z) (`KismetMathLibrary.BreakVector` (`SceneComponent.RelativeLocation` _elevator4)))
  (bind (_relativelocation_x_2 _relativelocation_y_2 _relativelocation_z_2) (`KismetMathLibrary.BreakVector` (`SceneComponent.RelativeLocation` _elevator4_2)))
  ;[1 0 0.1888 1 94] Elevator movement
  (`/Engine/EditorBlueprintResources/StandardMacros.DoOnce` false :!label _label_6
    (:`Completed`
      (if (`PrimitiveComponent.IsOverlappingComponent` (`self.ElevatorStart4`) (`self.ElevatorCube`))
        (`KismetSystemLibrary.Delay` 1.5)
        (`KismetSystemLibrary.MoveComponentTo` _elevator4_2 (`KismetMathLibrary.MakeVector` (+ _relativelocation_x_2 300.0) _relativelocation_y_2 _relativelocation_z_2) (`SceneComponent.RelativeRotation` _elevator4_2) false false 2.0)
        (`KismetSystemLibrary.Delay` 2.0)
        (`KismetSystemLibrary.MoveComponentTo` _elevator4 (`KismetMathLibrary.MakeVector` (+ _relativelocation_x -300.0) _relativelocation_y _relativelocation_z) (`SceneComponent.RelativeRotation` _elevator4) false false 2.0)))))

(event `self.ElevatorStart4.OnComponentEndOverlap`
  (params (OverlappedComponent :type "PrimitiveComponent Object Reference") (OtherActor :type "Actor Object Reference") (OtherComp :type "PrimitiveComponent Object Reference") (OtherBodyIndex :type Integer))
  ;[1 0 0.1888 1 94] Elevator movement
  (goto _label_6 :!via `Reset`))

(event `self.AnswerCollider4.OnComponentBeginOverlap`
  (params (OverlappedComponent :type "PrimitiveComponent Object Reference") (OtherActor :type "Actor Object Reference") (OtherComp :type "PrimitiveComponent Object Reference") (OtherBodyIndex :type Integer) (bFromSweep :type Boolean) (SweepResult :type "HitResult Structure (by ref)"))
  ;[0 0.5255 1 1 132] Answer logic
  (if (`self.Answer4Available`)
    (if (not (`self.Answered`))
      (`/Engine/EditorBlueprintResources/StandardMacros.DoOnce` false :!label _label_7
        (:`Completed`
          (`/Game/MarkS/UIX/MainWidget.ShowAnswerMessage` (`self.MainWidget`))
          (cast `Character` OtherActor)
          (`self.EnableInput` (`GameplayStatics.GetPlayerController` 0)))))))

(event `self.AnswerCollider3.OnComponentBeginOverlap`
  (params (OverlappedComponent :type "PrimitiveComponent Object Reference") (OtherActor :type "Actor Object Reference") (OtherComp :type "PrimitiveComponent Object Reference") (OtherBodyIndex :type Integer) (bFromSweep :type Boolean) (SweepResult :type "HitResult Structure (by ref)"))
  ;[0 0.5255 1 1 132] Answer logic
  (if (`self.Answer3Available`)
    (if (not (`self.Answered`))
      (`/Engine/EditorBlueprintResources/StandardMacros.DoOnce` false :!label _label_8
        (:`Completed`
          (`/Game/MarkS/UIX/MainWidget.ShowAnswerMessage` (`self.MainWidget`))
          (cast `Character` OtherActor)
          (`self.EnableInput` (`GameplayStatics.GetPlayerController` 0)))))))

(event `self.AnswerCollider4.OnComponentEndOverlap`
  (params (OverlappedComponent :type "PrimitiveComponent Object Reference") (OtherActor :type "Actor Object Reference") (OtherComp :type "PrimitiveComponent Object Reference") (OtherBodyIndex :type Integer))
  ;[0 0.5255 1 1 132] Answer logic
  (if (`self.Answer4Available`)
    (`/Game/MarkS/UIX/MainWidget.HideAnswerMessage` (`self.MainWidget`))
    (cast `Character` OtherActor)
    (`self.DisableInput` (`GameplayStatics.GetPlayerController` 0))
    (goto _label_7 :!via `Reset`)))

(event `self.AnswerCollider3.OnComponentEndOverlap`
  (params (OverlappedComponent :type "PrimitiveComponent Object Reference") (OtherActor :type "Actor Object Reference") (OtherComp :type "PrimitiveComponent Object Reference") (OtherBodyIndex :type Integer))
  ;[0 0.5255 1 1 132] Answer logic
  (if (`self.Answer3Available`)
    (`/Game/MarkS/UIX/MainWidget.HideAnswerMessage` (`self.MainWidget`))
    (cast `Character` OtherActor)
    (`self.DisableInput` (`GameplayStatics.GetPlayerController` 0))
    (goto _label_8 :!via `Reset`)))

(event `self.Box4.OnComponentBeginOverlap`
  (params (OverlappedComponent :type "PrimitiveComponent Object Reference") (OtherActor :type "Actor Object Reference") (OtherComp :type "PrimitiveComponent Object Reference") (OtherBodyIndex :type Integer) (bFromSweep :type Boolean) (SweepResult :type "HitResult Structure (by ref)"))
  ;[0 0.5255 1 1 132] Answer logic
  (if (`PrimitiveComponent.IsOverlappingComponent` (`self.Box4`) (`self.AnswerCube4`))
    (set `self.Answer4Available` true)
    (`PrimitiveComponent.SetMaterial` (`self.Button4`) 0 "/Game/MarkS/Materials/Red.Red")))

(event `self.Box3.OnComponentBeginOverlap`
  (params (OverlappedComponent :type "PrimitiveComponent Object Reference") (OtherActor :type "Actor Object Reference") (OtherComp :type "PrimitiveComponent Object Reference") (OtherBodyIndex :type Integer) (bFromSweep :type Boolean) (SweepResult :type "HitResult Structure (by ref)"))
  ;[0 0.5255 1 1 132] Answer logic
  (if (`PrimitiveComponent.IsOverlappingComponent` (`self.Box3`) (`self.AnswerCube3`))
    (set `self.Answer3Available` true)
    (`PrimitiveComponent.SetMaterial` (`self.Button3`) 0 "/Game/MarkS/Materials/Red.Red")))

(event `self.Box4.OnComponentEndOverlap`
  (params (OverlappedComponent :type "PrimitiveComponent Object Reference") (OtherActor :type "Actor Object Reference") (OtherComp :type "PrimitiveComponent Object Reference") (OtherBodyIndex :type Integer))
  ;[0 0.5255 1 1 132] Answer logic
  (if (not (`PrimitiveComponent.IsOverlappingComponent` (`self.Box4`) (`self.AnswerCube4`)))
    (set `self.Answer4Available` false)
    (`PrimitiveComponent.SetMaterial` (`self.Button4`) 0 "/Game/MarkS/Materials/Yellow.Yellow")))

(event `self.Box3.OnComponentEndOverlap`
  (params (OverlappedComponent :type "PrimitiveComponent Object Reference") (OtherActor :type "Actor Object Reference") (OtherComp :type "PrimitiveComponent Object Reference") (OtherBodyIndex :type Integer))
  ;[0 0.5255 1 1 132] Answer logic
  (if (not (`PrimitiveComponent.IsOverlappingComponent` (`self.Box3`) (`self.AnswerCube3`)))
    (set `self.Answer3Available` false)
    (`PrimitiveComponent.SetMaterial` (`self.Button3`) 0 "/Game/MarkS/Materials/Orange.Orange")))

(fn `OpenCloseDoor`
  (params (Open :type Boolean) (Door :type "StaticMeshComponent Object Reference"))
  (returns (OutDoor :type "StaticMeshComponent Object Reference") (RelativeRotation :type "Rotator Structure") (ReturnValue :type "Vector Structure"))
  (bind (_relativelocation_x _relativelocation_y _relativelocation_z) (`KismetMathLibrary.BreakVector` (`SceneComponent.RelativeLocation` Door)))
  (bind (_relativelocation_x_2 _relativelocation_y_2 _relativelocation_z_2) (`KismetMathLibrary.BreakVector` (`SceneComponent.RelativeLocation` Door)))
  (bind _relativerotation (`SceneComponent.RelativeRotation` Door))
  (if Open
    (return Door _relativerotation (`KismetMathLibrary.MakeVector` (+ (`self.MoveDistance`) _relativelocation_x_2) _relativelocation_y_2 _relativelocation_z_2))
    (else
      (return Door _relativerotation (`KismetMathLibrary.MakeVector` (- _relativelocation_x (`self.MoveDistance`)) _relativelocation_y _relativelocation_z)))))

(fn `UserConstructionScript`)