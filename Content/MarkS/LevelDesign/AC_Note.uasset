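; Pickup note actor that the player collects with the Interact input to reveal a note in the UI.
; Overlapping its trigger A fetches the main widget from the first FirstPersonCharacter, shows the pickup prompt and enables input on the actor for Characters.
; Leaving hides the prompt, and for Characters disables input and resets the DoOnce gate on entry.
; Pressing Interact destroys the actor and tells the widget to reveal the note.
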(event `self.a.OnComponentBeginOverlap`
  (params (OverlappedComponent :type "PrimitiveComponent Object Reference") (OtherActor :type "Actor Object Reference") (OtherComp :type "PrimitiveComponent Object Reference") (OtherBodyIndex :type Integer) (bFromSweep :type Boolean) (SweepResult :type "HitResult Structure (by ref)"))
  (bind _outactors (`GameplayStatics.GetAllActorsOfClass` "/Game/MarkS/Characters/FirstPersonCharacter.FirstPersonCharacter_C"))
  (set `self.MainWidget` (`/Game/MarkS/Characters/FirstPersonCharacter.Widget` (`|GetArrayItem` _outactors)))
  (`/Engine/EditorBlueprintResources/StandardMacros.DoOnce` false :!label _label
    (:`Completed`
      (`/Game/MarkS/UIX/MainWidget.ShowPickUp` (`self.MainWidget`))
      (cast `Character` OtherActor)
      (`self.EnableInput` (`GameplayStatics.GetPlayerController` 0)))))

(event `self.a.OnComponentEndOverlap`
  (params (OverlappedComponent :type "PrimitiveComponent Object Reference") (OtherActor :type "Actor Object Reference") (OtherComp :type "PrimitiveComponent Object Reference") (OtherBodyIndex :type Integer))
  (`/Game/MarkS/UIX/MainWidget.HidePickUp` (`self.MainWidget`))
  (cast `Character` OtherActor)
  (`self.DisableInput` (`GameplayStatics.GetPlayerController` 0))
  (goto _label :!via `Reset`))

(event `InputAction|Interact`
  (params (Key :type "Key Structure"))
  (:`Pressed`
    (`self.K2_DestroyActor`)
    (`/Game/MarkS/UIX/MainWidget.RevealNote` (`self.MainWidget`))))

(fn `UserConstructionScript`)